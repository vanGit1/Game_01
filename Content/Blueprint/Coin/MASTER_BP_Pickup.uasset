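; Master pickup Blueprint for a coin that spins in place and is collected when the player overlaps its collision sphere.
; A looping timeline rotates the coin a full turn around yaw.
; On the first BP_Player overlap, a second timeline lerps it from its start location to the player's moving position while shrinking it to zero, creating a magnet effect.
; When that finishes, it adds BaseValue via AddCoinExperience, plays the pickup sound and destroys itself.
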(event OnComponentBeginOverlap(Sphere_Collision)
  (params (OverlappedComponent :type Primitive%20Component%20Object%20Reference) (OtherActor :type Actor%20Object%20Reference) (OtherComp :type Primitive%20Component%20Object%20Reference) (OtherBodyIndex :type Integer) (bFromSweep :type Boolean) (SweepResult :type Hit%20Result%20Structure%20%28by%20ref%29))
  ;[0 0 0 1 14] При перекрытии получаем ссылку на игрока
  (bind _asbp_player (Utilities|Casting|CastToBP_Player OtherActor))
  (Variables|Default|SetPlayer%20Ref _asbp_player)
  (Utilities|FlowControl|DoOnce false
    (:Completed
      ;[0 0 0 1 13] Coin
      (bind _alpha (Timeline|ShrinkCoinToPlayer PlayFromStart)
        (:Update
          (Transformation|SetActorLocation (Math|Vector|Lerp(Vector) (Variables|Default|GetStartingPickupLocation) (Transformation|GetActorLocation (Variables|Default|GetPlayer%20Ref)) _alpha) false false)
          (Transformation|SetActorScale3D (Math|Vector|Lerp(Vector) "1.000000,1.000000,1.000000" "0, 0, 0" _alpha)))
        (:Finished
          ;;[0.01427 0.0734 0.0946 1 13] Перед уничтожение вызовем функцию подсчета монет
          (Default|AddCoinExperience (Variables|Default|GetPlayer%20Ref) (Variables|Default|GetBase%20Value))
          ;;[0.04915 0.04915 0.04915 1 13] Звук подбора монеты
          (Audio|PlaySoundatLocation "/Game/Audio/Coin.Coin" (Transformation|GetActorLocation) "0, 0, 0" 1.0 1.0 0.0 0 0 0 0)
          (Actor|DestroyActor))))))

(event EventBeginPlay
  ;[0 0 0 1 13] получаем начальное  местоположение монеты
  (Variables|Default|SetStartingPickupLocation (Transformation|GetActorLocation))
  ;[0 0 0] Spin the coin 360
  (bind _z (Timeline|Rotation360 PlayFromStart)
    (:Update
      (Transformation|SetActorRotation (Math|Rotator|MakeRotator 0.0 0.0 (Math|Float|Lerp 0.0 3.6e+02 _z))))
    (:Finished
      (Timeline|Rotation360 PlayFromStart))))

(fn ConstructionScript)