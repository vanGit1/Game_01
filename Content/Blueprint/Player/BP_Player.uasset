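; BP_Player is the player actor, moving on world X/Y axes via Enhanced Input and turning toward the cursor.
; Each Tick, cursor traces on the Visibility channel drive the actor's rotation and position the crosshair mesh.
; A looping timer started at BeginPlay automatically spawns Spell_Fire at the player's transform.
; Events subtract enemy damage and update the health widget's percentage, or add coin experience and print the total.
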(event Custom|AddCoinExperience
  (params (PickUp%20Value :type Float%20%28double-precision%29))
  ;[0 0 0] Подсчет монет
  (bind _output_get (Variables|Default|SetExperienceCoin (+ (Variables|Default|GetExperienceCoin) PickUp%20Value)))
  (Development|PrintString (Utilities|String|ToString(Float) _output_get)))

(event Custom|Get%20Hurt%20and%20Update%20Health
  (params (EnemyDamage :type Float%20%28double-precision%29))
  ;[0 0 0 1 12] Событие считает получаемый урон
  ;;[0.1082 0.1082 0.1082 1 11] Вычитает урон из здоровья игрока
  ;;[0.1037 0.1037 0.1037 1 11] Устанавливает значения здоровья после получения урона, и делит его на 100 (PlayerHealthMax) для получения процента для Progress bar в виджете
  (bind _output_get (Variables|Default|SetPlayer_Health (- (Variables|Default|GetPlayer_Health) EnemyDamage)))
  ;[0 0 0 1 11] вызов события, которое обновить процент
  (Default|UpdatePercent (Variables|Default|GetRef_Widget) (/ _output_get (Variables|Default|GetPlayer_HealthMax))))

(event Input|EnhancedActionEvents|EnhancedInputActionIA_Movement
  (params (ActionValue :type Vector%202D%20Structure) (ElapsedSeconds :type Float%20%28double-precision%29) (TriggeredSeconds :type Float%20%28double-precision%29) (InputAction :type Input%20Action%20Object%20Reference :default "/Game/Blueprint/Player/IA_Movement.IA_Movement"))
  (Pawn|Input|AddMovementInput "1.000000,0.000000,0.000000" (.x ActionValue) false)
  (Pawn|Input|AddMovementInput "0.000000,1.000000,0.000000" (.y ActionValue) false))

(event EventBeginPlay
  ;[0.1413 0.1351 0.1946] Add mapping context
  (Input|AddMappingContext (PlayerController|LocalPlayerSubsystems|GetEnhancedInputLocalPlayerSubsystem (Game|GetPlayerController 0)) "/Game/Blueprint/Player/IMC_Player.IMC_Player" 0 "(bIgnoreAllPressedKeysUntilRelease=True,bForceImmediately=False,bNotifyUserSettings=False)")
  ;[0 0 0 1 12] виджет здоровья игрока
  (bind _returnvalue (UserInterface|CreateWidget "/Game/Blueprint/Player/Widgets/WBP_PlayerHealth.WBP_PlayerHealth_C"))
  (bind _output_get (Variables|Default|SetRef_Widget _returnvalue))
  (UserInterface|Viewport|AddtoViewport _output_get 0)
  ;[0 0 0 1 13] функция, которая задаёт таймер для выполнения другой функции (SpellSpawnFireball) через определенный интервал времени.
  ; Внутри функция, которая будет создавать актера каждые 0.25сек.
  (Utilities|Time|SetTimerbyFunctionName 0 "SpellSpawnFireball" 0.25 true))

(event EventTick
  (params (DeltaSeconds :type Float%20%28single-precision%29))
  (bind _returnvalue (Transformation|GetActorLocation))
  (bind _returnvalue_2 (Game|GetPlayerController 0))
  (bind _hitresult (Game|Player|GetHitResultUnderCursorbyChannel _returnvalue_2 "TraceTypeQuery1" true))
  (bind _location (Collision|BreakHitResult _hitresult))
  ;[0 0 0] следование за курсором
  (Transformation|SetActorRotation (Math|Rotator|FindLookatRotation (Math|Vector|MakeVector (.x _returnvalue) (.y _returnvalue) 0.0) (Math|Vector|MakeVector (.x _location) (.y _location) 0.0)))
  ;;[0 0 0 1 14] поместить объект в место курсора
  (Transformation|SetWorldLocation (Variables|Default|GetMesh_Crosshair) (Math|Vector|MakeVector (.x _location) (.y _location) 0.0) true false))

(fn ConstructionScript)

(fn SpellSpawnFireball
  ;[0 0 0 1 15] создать нового актера на основе класса (Spell fire), и место появление в месторасположении игрока
  (Game|SpawnActorfromClass "/Game/Blueprint/Player/Spells/Spell_Fire.Spell_Fire_C" (Transformation|GetActorTransform) "Undefined" "MultiplyWithRoot" 0 0))