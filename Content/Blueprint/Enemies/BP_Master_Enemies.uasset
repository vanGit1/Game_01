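; Master enemy Blueprint, with slime mesh and sound, that chases the player and deals contact damage.
; A delayed AIMoveTo loop drives pursuit, while sphere overlap hurts BP_Player through a DoOnce cooldown.
; SpellCollisionEvent subtracts randomized damage, updates the health widget, then destroys the enemy or plays damage text, whose random roll is separate.
; Surviving hits also flash white via a timeline driving a dynamic material created in the Construction Script.
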(event OnComponentBeginOverlap(Sphere_Collision)
  (params (OverlappedComponent :type Primitive%20Component%20Object%20Reference) (OtherActor :type Actor%20Object%20Reference) (OtherComp :type Primitive%20Component%20Object%20Reference) (OtherBodyIndex :type Integer) (bFromSweep :type Boolean) (SweepResult :type Hit%20Result%20Structure%20%28by%20ref%29))
  ;[0 0 0] При перекрытии вызвать событие для обновления здоровья игрока
  (bind _asbp_player (Utilities|Casting|CastToBP_Player OtherActor))
  (Utilities|FlowControl|DoOnce false :!label _label
    (:Completed
      (Default|GetHurtandUpdateHealth _asbp_player (Variables|Default|GetEnemy%20Damage))
      (Utilities|FlowControl|Delay 0.2)
      (goto _label Reset))))

(event Custom|EnemyFlasgingWhite
  ;[0 0 0] Dynamic material
  (bind (_direction _scalar) (Timeline|Flashing PlayFromStart)
    (:Update
      (Rendering|Material|SetScalarParameterValue (Variables|Default|GetRef%20Material) "FlashEmission" _scalar :!class /Script/Engine.MaterialInstanceDynamic))))

(event EventBeginPlay
  ;[0 0 0] Ссылка на виждет
  (bind _aswbp_enemy_health (Utilities|Casting|CastToWBP_EnemyHealth (UserInterface|GetWidget (Variables|Default|GetHealthWidget))))
  (Variables|Default|SetWidget%20ref _aswbp_enemy_health)
  ;[0 0 0 1 11] управление движением и поведением искусственного интеллекта в игре
  (AI|AIMoveTo self "0, 0, 0" (Game|GetPlayerCharacter 0) 5e+01 false :!label _label
    (:then
      ;[0 0 0 1 11] Задержка перед преследованием
      (Utilities|FlowControl|Delay 0.2)
      (goto _label))))

(event EventSpellCollisionEvent
  (params (SpellDamageInput :type Float%20%28double-precision%29))
  (bind _returnvalue (Math|Random|RandomFloatinRange -2.0 3.0))
  (bind _returnvalue_2 (+ SpellDamageInput _returnvalue))
  ;[0 0 0 1 14] Вызвать событие из интерфейса и посчитать кол-во урона для Slime
  (bind _output_get (Variables|Default|SetEnemyHealth (- (Variables|Default|GetEnemyHealth) _returnvalue_2)))
  (Default|UpdateEnemyHealth (Variables|Default|GetWidget%20ref) (/ _output_get (Variables|Default|GetEnemyHealthMax)))
  ;[0 0 0 1 14] звук при попадании
  (Audio|PlaySoundatLocation "/Game/Audio/SlimeImpact.SlimeImpact" (Transformation|GetActorLocation) "0, 0, 0" 1.0 1.0 0.0 0 0 0 0)
  ;[0 0 0 1 14] Событие смерти
  (if (<= (Variables|Default|GetEnemyHealth) 0.0)
    (Actor|DestroyActor)
    (else
      ;[0 0 0 1 14] Вызов динамического материала
      (CallFunction|EnemyFlasgingWhite)
      ;[0 0 0 1 14] Вызов анимации текста
      (Default|PlayDMGTextAnim (Variables|Default|GetWidget%20ref) _returnvalue_2))))

(fn ConstructionScript
  ;[0 0 0] Создаёт динамический материал
  ;;[0.1082 0.1082 0.1082 1 14] создаёт копию материала во время игры
  (bind _returnvalue (Rendering|Material|CreateDynamicMaterialInstance "/Game/Blueprint/Enemies/Textures/MI_Slime_Inst.MI_Slime_Inst" "None" "None" :!class /Script/Engine.KismetMaterialLibrary))
  ;;[0.03551 0.03551 0.03551 1 14] Сохраняет значение материала в переменную
  (bind _output_get (Variables|Default|SetRef%20Material _returnvalue))
  ;;[0.05369 0.05369 0.05369 1 14] Установить материал для выбранного объекта
  (Rendering|Material|SetMaterial (Variables|Default|GetMesh_Slime) 0 _output_get))